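; Sound gun actor that plays Niagara absorb and assign effects at the gun mesh and shows a widget on it.
; Absorb VFX stays attached until explicitly destroyed; assign VFX detaches in world space and auto-destroys.
; The two spawn events use oppositely named template variables.
; Tick checks validity until it can feed the widget's render target into a dynamic material on one mesh slot.
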(event Custom|SpawnAbsorbVFX
  (params (Rotation :type Rotator))
  (bind _handwgun (Variables|Default|GetHandwGun))
  (bind _returnvalue (Niagara|SpawnSystemAttached (Variables|Default|GetAssignNiagaraVFX) _handwgun "None" (Transformation|GetWorldLocation _handwgun) Rotation "KeepWorldPosition" false))
  (Variables|Default|SetActiveAbsorbVFX _returnvalue))

(event Custom|DestroyAbsorbVFX
  (Components|DestroyComponent (Variables|Default|GetActiveAbsorbVFX)))

(event Custom|SpawnAssignVFX
  (params (Rotation :type Rotator))
  (bind _handwgun (Variables|Default|GetHandwGun))
  (bind _returnvalue (Niagara|SpawnSystemAttached (Variables|Default|GetAbsorbNiagaraVFX) _handwgun "None" (Transformation|GetWorldLocation _handwgun) Rotation "KeepWorldPosition" true))
  (Transformation|DetachFromComponent _returnvalue "KeepWorld" "KeepWorld" "KeepWorld" true))

(event EventBeginPlay)

(event Collision|EventActorBeginOverlap
  (params (OtherActor :type Actor%20Object%20Reference)))

(event EventTick
  (params (DeltaSeconds :type Float%20%28single-precision%29))
  (bind _widget (Variables|Default|GetWidget))
  (bind _returnvalue (Class|WidgetComponent|GetRenderTarget _widget))
  (Utilities|IsValid 0
    (:Is%20Not%20Valid
      (Utilities|IsValid _returnvalue
        (:Is%20Valid
          (bind _returnvalue_2 (Rendering|Material|CreateDynamicMaterialInstance (Variables|Default|GetHandwGun) 3 "/Game/FirstPerson/NewMaterial.NewMaterial" "None" :!class /Script/Engine.PrimitiveComponent))
          (bind _output_get (Variables|Default|SetGunDMI _returnvalue_2))
          (Rendering|Material|SetTextureParameterValue _output_get "UI_Texture" _returnvalue)
          (Rendering|Material|SetMaterial (Variables|Default|GetHandwGun) 3 _output_get))))))

(fn ConstructionScript)