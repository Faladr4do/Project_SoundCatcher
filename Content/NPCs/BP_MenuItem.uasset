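; BP_MenuItem is an actor with a static mesh that acts as a mouse-interactive menu item, currently at a placeholder stage.
; Cursor hover toggles Render Custom Depth on the mesh, which allows a post-process highlight, and prints a debug string on enter and exit.
; Clicking only prints a debug message; BeginPlay, overlap and construction script are empty, and an enum variable is unused.
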(event EventBeginPlay)

(event MouseInput|EventActorOnClicked
  (params (ButtonPressed :type Key%20Structure :default "None"))
  (Development|PrintString "Click"))

(event Collision|EventActorBeginOverlap
  (params (OtherActor :type Actor%20Object%20Reference)))

(event MouseInput|EventActorBeginCursorOver
  (Rendering|SetRenderCustomDepth (Variables|Default|GetStaticMesh) true)
  (Development|PrintString "Hover"))

(event MouseInput|EventActorEndCursorOver
  (Rendering|SetRenderCustomDepth (Variables|Default|GetStaticMesh) false)
  (Development|PrintString "NotHover"))

(fn ConstructionScript)