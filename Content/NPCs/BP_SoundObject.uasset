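; BP_SoundObject is an interactable object that holds swappable sounds and checks whether the equipped one matches its original.
; Adding or removing sounds updates the Audio component's wave and trigger parameters, while interacting replays it; match results are only printed.
; Selection toggles a custom-depth highlight and a WB_SoundObjectStats widget component showing name and sound.
; Only the first array entry plays; a second is merely detected.
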(event Custom|AddSound
  (params (newSound :type Array%20of%20Sound%20Wave%20Object%20References))
  (bind _output_get (Variables|Default|SetEquippedSounds newSound))
  (if (== (Utilities|Array|Get(acopy) (Variables|Default|GetOriginalSound)) (Utilities|Array|Get(acopy) (Variables|Default|GetEquippedSounds)))
    (Development|PrintString "Right Sound")
    (else
      (Development|PrintString "Bad Sound")))
  (CallFunction|ChangeSound _output_get true)
  (bind (_newparam _newparam1) (CallFunction|UpdateStats (Variables|Default|GetEquippedSound)))
  (Default|UpdateSound _newparam _newparam1))

(event Custom|Remove%20Sound
  (bind _equippedsounds (Variables|Default|GetEquippedSounds))
  (for (_ _array_index) _equippedsounds
    (Utilities|Array|RemoveIndex _equippedsounds _array_index))
  (Development|PrintString "Removed Sound")
  (CallFunction|ChangeSound 0 true)
  (bind (_newparam _newparam1) (CallFunction|UpdateStats (Variables|Default|GetEquippedSound)))
  (Default|UpdateSound _newparam _newparam1))

(event Custom|Interact
  (bind _equippedsounds (Variables|Default|GetEquippedSounds))
  (bind _output (Utilities|Array|Get(acopy) _equippedsounds))
  (Utilities|IsValid _output
    (:Is%20Valid
      (if (== _output (Utilities|Array|Get(acopy) (Variables|Default|GetOriginalSound)))
        (Development|PrintString "InteractionComplete"))
      (Class|AudioParameterControllerInterface|SetTriggerParameter (Variables|Default|GetAudio) "Replay"))))

(event Custom|OnSoundObjectSelect
  (bind (_newparam _newparam1) (CallFunction|UpdateStats (Utilities|Array|Get(acopy) (Variables|Default|GetEquippedSounds))))
  (Default|UpdateSound _newparam _newparam1)
  (Rendering|SetRenderCustomDepth (Variables|Default|GetMesh) true)
  (CallFunction|ShowStats true))

(event Custom|OnSoundObjectDeselect
  (Rendering|SetRenderCustomDepth (Variables|Default|GetMesh) false)
  (CallFunction|ShowStats false))

(event EventBeginPlay
  (bind _equippedsounds (Variables|Default|GetEquippedSounds))
  (Utilities|IsValid (Utilities|Array|Get(acopy) _equippedsounds)
    (:Is%20Valid
      (CallFunction|ChangeSound _equippedsounds false))
    (:Is%20Not%20Valid
      _))
  (CallFunction|ShowStats false)
  (bind (_newparam _newparam1) (CallFunction|UpdateStats (Utilities|Array|Get(acopy) (Variables|Default|GetOriginalSound))))
  (Default|UpdateName _newparam _newparam1)
  (bind (_newparam_2 _newparam1_2) (CallFunction|UpdateStats (Utilities|Array|Get(acopy) (Variables|Default|GetEquippedSounds))))
  (Default|UpdateSound _newparam_2 _newparam1_2))

(fn ConstructionScript)

(fn ChangeSound
  (params (NewSound :type Array%20of%20Sound%20Wave%20Object%20References) (Play :type Boolean))
  (bind _audio (Variables|Default|GetAudio))
  (Class|AudioComponent|SetWaveParameter _audio "AudioLoop" (Utilities|Array|Get(acopy) NewSound))
  (if Play
    (Class|AudioParameterControllerInterface|SetTriggerParameter _audio "Replay")
    (Utilities|IsValid (Utilities|Array|Get(acopy) NewSound 1)
      (:Is%20Valid
        (Development|PrintString "has secondary sound"))
      (:Is%20Not%20Valid
        (Development|PrintString "doesnt have secondary sound")))))

(fn ShowStats
  (params (Show :type Boolean))
  (bind _stats (Variables|Default|GetStats))
  (Utilities|FlowControl|Sequence
    (:then_0
      (Rendering|SetVisibility _stats Show false))
    (:then_1
      (Rendering|SetVisibility _stats Show false))))

(fn UpdateStats
  (params (stat :type Sound%20Wave%20Object%20Reference))
  (bind _aswb_sound_object_stats (Utilities|Casting|CastToWB_SoundObjectStats (UserInterface|GetWidget (Variables|Default|GetStats))))
  (return _aswb_sound_object_stats (Utilities|GetDisplayName stat)))