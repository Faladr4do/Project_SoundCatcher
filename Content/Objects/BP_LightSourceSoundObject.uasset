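; Interactable sound object with a point light whose visibility depends on the sound data equipped in it.
; On PressInteract, a valid EquippedSound that casts to PDA_LightSourceSoundObjects sets the light's visibility from IsTurnedON, read before the press is forwarded to that data asset.
; Other sound types receive the forwarded press without any change to the light.
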(event EventBeginPlay
  (|CallParentFunction) ; This node is disabled and will not be called.\nDrag off pins to build functionality.
)

(event Collision|EventActorBeginOverlap
  (params (OtherActor :type Actor%20Object%20Reference)))

(event EventTick
  (params (DeltaSeconds :type Float%20%28single-precision%29)))

(event EventPressInteract
  (bind _equippedsound (Variables|Default|GetEquippedSound))
  (bind _pointlight (Variables|Default|GetPointLight))
  (Utilities|IsValid _equippedsound
    (:Is%20Valid
      (bind _aspda_light_source_sound_objects (Utilities|Casting|CastToPDA_LightSourceSoundObjects _equippedsound)
        (:then
          (if (Variables|/Game/DataAssets/PDA_LightSourceSoundObjects.PDA_LightSourceSoundObjects_C|GetisTurnedON _aspda_light_source_sound_objects)
            (Rendering|SetVisibility _pointlight true false)
            (else
              (Rendering|SetVisibility _pointlight false false)))
          (bind _aspda_light_source_sound_objects_2 (Utilities|Casting|CastToPDA_LightSourceSoundObjects (Variables|Default|GetEquippedSound)))
          (Default|PressInteract _aspda_light_source_sound_objects_2))
        (:CastFailed
          (Default|PressInteract _equippedsound))))))

(fn ConstructionScript
  (|CallParentFunction))