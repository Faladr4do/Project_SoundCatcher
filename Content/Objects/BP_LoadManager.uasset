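; BP_LoadManager shows a loading screen while it loads and opens the level set in LevelToLoad.
; On BeginPlay it adds a WBP_LoadingScreen widget to the viewport and starts an async load of the level asset.
; When the load completes, it opens the level by object reference, removes the widget and requests garbage collection.
; An unconnected branch that reads the current level from BP_GameInstance never runs.
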(event EventBeginPlay
  (bind _returnvalue (Game|ConstructObjectfromClass (Game|GetPlayerController 0) "/Game/UI/WBP_LoadingScreen.WBP_LoadingScreen_C"))
  (bind _output_get (Variables|Default|SetLoadingWidget _returnvalue))
  (UserInterface|Viewport|AddtoViewport _output_get 0)
  (Utilities|AsyncLoadAsset (Variables|Default|GetLevelToLoad)
    (:Completed
      (Game|OpenLevel(byObjectReference) (Variables|Default|GetLevelToLoad))
      (Widget|RemovefromParent (Variables|Default|GetLoadingWidget))
      (Utilities|Platform|CollectGarbage))))

(fn ConstructionScript)