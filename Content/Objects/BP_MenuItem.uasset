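; BP_MenuItem is a clickable 3D menu actor that either opens the Tutorial level or quits the game, depending on an enum variable.
; Cursor hover toggles the mesh's custom depth rendering, with a stencil value set per item type at BeginPlay.
; A text label starts hidden and appears on hover only for the Tutorial variant.
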(event EventBeginPlay
  (bind _staticmesh (Variables|Default|GetStaticMesh))
  (if (Utilities|Enum|Equal(Enum) (Variables|Default|GetNewVar) "NewEnumerator0")
    (Rendering|SetCustomDepthStencilValue _staticmesh 3)
    (else
      (Rendering|SetCustomDepthStencilValue _staticmesh 2)))
  (Rendering|SetVisibility (Variables|Default|GetTextRender) false false))

(event MouseInput|EventActorOnClicked
  (params (ButtonPressed :type Key%20Structure :default "None"))
  (if (Utilities|Enum|Equal(Enum) (Variables|Default|GetNewVar) "NewEnumerator0")
    (Game|OpenLevel(byName) "Tutorial")
    (else
      (Game|QuitGame 0 "Quit" false))))

(event MouseInput|EventActorBeginCursorOver
  (Rendering|SetRenderCustomDepth (Variables|Default|GetStaticMesh) true)
  (if (Utilities|Enum|Equal(Enum) (Variables|Default|GetNewVar) "NewEnumerator0")
    (Rendering|SetVisibility (Variables|Default|GetTextRender) true false)))

(event MouseInput|EventActorEndCursorOver
  (Rendering|SetRenderCustomDepth (Variables|Default|GetStaticMesh) false)
  (if (Utilities|Enum|Equal(Enum) (Variables|Default|GetNewVar) "NewEnumerator0")
    (Rendering|SetVisibility (Variables|Default|GetTextRender) false false)))

(fn ConstructionScript)