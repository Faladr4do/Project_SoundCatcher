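; World object that holds a swappable sound data asset and checks whether it matches the object's original sound.
; Feeds the asset's waves into looping Passive and one-shot Audio components, with gameplay tags choosing press/hold behavior for default, toggle, radio and light types.
; Selection boosts volume, shows HUD options and outlines incorrect objects via custom depth.
; The player's focus mode muffles unselected objects through volume and source effect chains.
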(event Custom|AddSound
  (params (newSound :type PDA%20Sound%20Objects%20Object%20Reference))
  (Variables|Default|SetEquippedSound newSound)
  (CallFunction|UpdateSound)
  (CallFunction|CheckSoundCompatible)
  (|SwitchGameplayTag (Variables|/Game/DataAssets/PDA_SoundObjects.PDA_SoundObjects_C|GetObjectType (Variables|Default|GetEquippedSound))
    (:SoundObjects
      (CallFunction|PlayInteractiveSound)
      (CallFunction|PlayPassiveSound)
      (bind _ashud_test (Utilities|Casting|CastToHUD_Test (HUD|GetHUD (Game|GetPlayerController 0)) :!label _label))
      (Default|ShowInteractionOptions _ashud_test (Variables|Default|GetEquippedSound)))
    (:SoundObjects.Toggle
      (bind _aspda_toggle_sound_objects (Utilities|Casting|CastToPDA_ToggleSoundObjects (Variables|Default|GetEquippedSound)))
      (if (Variables|/Game/DataAssets/PDA_ToggleSoundObjects.PDA_ToggleSoundObjects_C|GetisTurnedOn _aspda_toggle_sound_objects)
        (bind _delay (CallFunction|PlayInteractiveSound (Variables|/Game/DataAssets/PDA_ToggleSoundObjects.PDA_ToggleSoundObjects_C|GetTurnOnSound _aspda_toggle_sound_objects)))
        (Utilities|FlowControl|Delay _delay)
        (CallFunction|PlayPassiveSound)
        (goto _label)))
    (:SoundObjects.Toggle.Radio
      (bind _aspda_music_player (Utilities|Casting|CastToPDA_MusicPlayer (Variables|Default|GetEquippedSound)))
      (if (Variables|/Game/DataAssets/PDA_ToggleSoundObjects.PDA_ToggleSoundObjects_C|GetisTurnedOn _aspda_music_player)
        (bind _delay_2 (CallFunction|PlayInteractiveSound (Variables|/Game/DataAssets/PDA_MusicPlayer.PDA_MusicPlayer_C|GetChangeMusicSound _aspda_music_player)))
        (Utilities|FlowControl|Delay (/ _delay_2 2.0))
        (CallFunction|PlayPassiveSound)
        (goto _label)))
    (:SoundObjects.Toggle.Light
      (bind _aspda_toggle_sound_objects_2 (Utilities|Casting|CastToPDA_ToggleSoundObjects (Variables|Default|GetEquippedSound)))
      (if (Variables|/Game/DataAssets/PDA_ToggleSoundObjects.PDA_ToggleSoundObjects_C|GetisTurnedOn _aspda_toggle_sound_objects_2)
        (bind _delay_3 (CallFunction|PlayInteractiveSound (Variables|/Game/DataAssets/PDA_ToggleSoundObjects.PDA_ToggleSoundObjects_C|GetTurnOnSound _aspda_toggle_sound_objects_2)))
        (Utilities|FlowControl|Delay _delay_3)
        (goto _label)))))

(event Custom|Remove%20Sound
  (Variables|Default|SetEquippedSound 0)
  (CallFunction|UpdateSound)
  (CallFunction|CheckSoundCompatible)
  (bind _ashud_test (Utilities|Casting|CastToHUD_Test (HUD|GetHUD (Game|GetPlayerController 0))))
  (Default|HideInteractionOptions _ashud_test)
  (CallFunction|ResetMyDoOnce))

(event Custom|PressInteract
  (bind _equippedsound (Variables|Default|GetEquippedSound))
  (Utilities|IsValid _equippedsound
    (:Is%20Valid
      (Utilities|FlowControl|DoOnce false
        (:Completed
          (|SwitchGameplayTag (Variables|/Game/DataAssets/PDA_SoundObjects.PDA_SoundObjects_C|GetObjectType _equippedsound)
            (:SoundObjects
              (Utilities|DefaultPressAction
                (:Completed
                  _)))
            (:SoundObjects.Toggle.Radio
              (Utilities|RadioPressAction)))
          (CallFunction|ResetMyDoOnce))))))

(event Custom|OnSoundObjectSelect
  (Variables|Default|SetSelected true)
  (bind _ashud_test (Utilities|Casting|CastToHUD_Test (HUD|GetHUD (Game|GetPlayerController 0))))
  (Default|ShowInteractionOptions _ashud_test (Variables|Default|GetEquippedSound))
  (CallFunction|SetOverallSound 1.4)
  (if (not (Variables|Default|GetbIsSoundCorrect))
    (for _array_element (Actor|GetComponentsByClass "/Script/Engine.StaticMeshComponent")
      (Rendering|SetRenderCustomDepth _array_element true))))

(event Custom|OnSoundObjectDeselect
  (Variables|Default|SetSelected false)
  (CallFunction|SetOverallSound 1.0)
  (bind _ashud_test (Utilities|Casting|CastToHUD_Test (HUD|GetHUD (Game|GetPlayerController 0))))
  (Default|HideInteractionOptions _ashud_test)
  (for _array_element (Actor|GetComponentsByClass "/Script/Engine.StaticMeshComponent")
    (Rendering|SetRenderCustomDepth _array_element false)))

(event Custom|HoldInteract
  (bind _equippedsound (Variables|Default|GetEquippedSound))
  (Utilities|IsValid _equippedsound
    (:Is%20Valid
      (|SwitchGameplayTag (Variables|/Game/DataAssets/PDA_SoundObjects.PDA_SoundObjects_C|GetObjectType _equippedsound)
        (:SoundObjects.Toggle
          (Utilities|ToggleHoldAction))
        (:SoundObjects.Toggle.Radio
          (Utilities|RadioHoldAction))
        (:SoundObjects.Toggle.Light
          (Utilities|ToggleHoldAction)))
      (CallFunction|ResetMyDoOnce))))

(event Custom|ResetMyDoOnce
  (Utilities|FlowControl|DoOnce false) ; enters at Reset
)

(event Custom|FocusMode
  (bind _passive (Variables|Default|GetPassive))
  (bind _audio (Variables|Default|GetAudio))
  (bind _passive_2 (Variables|Default|GetPassive))
  (bind _equippedsound (Variables|Default|GetEquippedSound))
  (bind _audio_2 (Variables|Default|GetAudio))
  (bind _soundeffectchain (Variables|/Game/DataAssets/PDA_SoundObjects.PDA_SoundObjects_C|GetSoundEffectChain _equippedsound))
  ;[0.15 0.15 0.15 0.5] Muffle SoundObject Sound
  (if (Variables|Default|GetSelected)
    ;[0.15 0.15 0.15 0.5] Unmuffle SoundObject Sound
    (Audio|Components|Audio|SetVolumeMultiplier _audio_2 1.0 :!class /Script/Engine.AudioComponent)
    (Variables|/Script/Engine.AudioComponent|SetSourceEffectChain _audio_2 _soundeffectchain)
    (Audio|Components|Audio|SetVolumeMultiplier _passive 1.0 :!class /Script/Engine.AudioComponent)
    (Variables|/Script/Engine.AudioComponent|SetSourceEffectChain _passive _soundeffectchain)
    (else
      (Audio|Components|Audio|SetVolumeMultiplier _audio 0.2 :!class /Script/Engine.AudioComponent)
      (Variables|/Script/Engine.AudioComponent|SetSourceEffectChain _audio "/Game/Sounds/NewFolder/MuffledSound.MuffledSound")
      (Audio|Components|Audio|SetVolumeMultiplier _passive_2 0.2 :!class /Script/Engine.AudioComponent)
      (Variables|/Script/Engine.AudioComponent|SetSourceEffectChain _passive_2 "/Game/Sounds/NewFolder/MuffledSound.MuffledSound"))))

(event Custom|FocusModeOff_Event
  (bind _passive (Variables|Default|GetPassive))
  (bind _equippedsound (Variables|Default|GetEquippedSound))
  (bind _audio (Variables|Default|GetAudio))
  (bind _soundeffectchain (Variables|/Game/DataAssets/PDA_SoundObjects.PDA_SoundObjects_C|GetSoundEffectChain _equippedsound))
  ;[0.15 0.15 0.15 0.5] Unmuffle SoundObject Sound
  (Audio|Components|Audio|SetVolumeMultiplier _audio 1.0 :!class /Script/Engine.AudioComponent)
  (Variables|/Script/Engine.AudioComponent|SetSourceEffectChain _audio _soundeffectchain)
  (Audio|Components|Audio|SetVolumeMultiplier _passive 1.0 :!class /Script/Engine.AudioComponent)
  (Variables|/Script/Engine.AudioComponent|SetSourceEffectChain _passive _soundeffectchain))

(event EventBeginPlay
  (bind _equippedsound (Variables|Default|GetEquippedSound))
  (Utilities|FlowControl|DelayUntilNextTick)
  (bind _asbp_first_person_character (Utilities|Casting|CastToBP_FirstPersonCharacter (Game|GetPlayerCharacter 0)))
  (bind _output_get (Variables|Default|SetAs%20BP%20First%20Person%20Character _asbp_first_person_character))
  (EventDispatchers|BindEventtoFocusModeon _output_get (delegate Custom|FocusMode))
  (EventDispatchers|AssignFocusModeOff _output_get (delegate Custom|FocusModeOff_Event))
  (CallFunction|ShowStats false)
  (CallFunction|UpdateSound)
  (CallFunction|PlayPassiveSound)
  (CallFunction|CheckSoundCompatible)
  (Default|Flush _equippedsound)
  (bind _aspda_toggle_sound_objects (Utilities|Casting|CastToPDA_ToggleSoundObjects _equippedsound))
  (Variables|/Game/DataAssets/PDA_ToggleSoundObjects.PDA_ToggleSoundObjects_C|SetisTurnedOn _aspda_toggle_sound_objects true)
  (Default|UpdateSoundObjectAsset _aspda_toggle_sound_objects))

(fn ConstructionScript)

(fn UpdateSound
  (bind _audio (Variables|Default|GetAudio))
  (bind _passive (Variables|Default|GetPassive))
  (bind _equippedsound (Variables|Default|GetEquippedSound))
  (bind _interactablesound (Variables|/Game/DataAssets/PDA_SoundObjects.PDA_SoundObjects_C|GetInteractableSound _equippedsound))
  (bind _passivesound (Variables|/Game/DataAssets/PDA_SoundObjects.PDA_SoundObjects_C|GetPassiveSound _equippedsound))
  (Utilities|IsValid _equippedsound
    (:Is%20Valid
      (Utilities|FlowControl|Sequence
        (:then_0
          ;[0.15 0.15 0.15 0.5] If Theres A Passive Sound Add It, Otherwise Clear Its Space And Play It Blank
          (Utilities|IsValid _passivesound
            (:Is%20Valid
              (Class|AudioComponent|SetWaveParameter _passive "AudioLoop" _passivesound)
              (Variables|/Script/Engine.AudioComponent|SetSourceEffectChain _passive (Variables|/Game/DataAssets/PDA_SoundObjects.PDA_SoundObjects_C|GetSoundEffectChain _equippedsound)))
            (:Is%20Not%20Valid
              (Class|AudioComponent|SetWaveParameter _passive "AudioLoop" :!label _label)
              (CallFunction|PlayPassiveSound))))
        (:then_1
          ;[0.15 0.15 0.15 0.5] If Theres An Interactable Sound Add It, Otherwise Clear Its Space And Play It Blank
          (Utilities|IsValid _interactablesound
            (:Is%20Valid
              (Class|AudioComponent|SetWaveParameter _audio "InteractiveAudio" _interactablesound))
            (:Is%20Not%20Valid
              (Class|AudioComponent|SetWaveParameter _audio "InteractiveAudio" :!label _label_2)
              (CallFunction|PlayInteractiveSound))))))
    (:Is%20Not%20Valid
      (Utilities|FlowControl|Sequence
        (:then_0
          (goto _label))
        (:then_1
          (goto _label_2))))))

(fn ShowStats
  (params (Show :type Boolean))
  (bind _stats (Variables|Default|GetStats))
  (Utilities|FlowControl|Sequence
    (:then_0
      (Rendering|SetVisibility _stats Show false))
    (:then_1
      (Rendering|SetVisibility _stats Show false))))

(fn UpdateStats
  (params (stat :type String))
  (bind _aswb_sound_object_stats (Utilities|Casting|CastToWB_SoundObjectStats (UserInterface|GetWidget (Variables|Default|GetStats))))
  (return _aswb_sound_object_stats stat))

(fn PlayInteractiveSound
  (params (NewSound :type Sound%20Wave%20Object%20Reference))
  (bind _equippedsound (Variables|Default|GetEquippedSound))
  (bind _audio (Variables|Default|GetAudio))
  (bind _interactablesound (Variables|/Game/DataAssets/PDA_SoundObjects.PDA_SoundObjects_C|GetInteractableSound _equippedsound))
  (Utilities|IsValid NewSound
    (:Is%20Valid
      (Class|AudioComponent|SetWaveParameter (Variables|Default|GetAudio) "InteractiveAudio" NewSound)
      (Audio|Components|Audio|Play _audio 0.0 :!label _label)
      (Utilities|IsValid _interactablesound
        (:Is%20Valid
          (return (- (Variables|/Script/Engine.SoundBase|GetDuration _interactablesound) 0.2)))))
    (:Is%20Not%20Valid
      (Utilities|IsValid _equippedsound
        (:Is%20Valid
          (Utilities|IsValid _interactablesound
            (:Is%20Valid
              (Class|AudioComponent|SetWaveParameter _audio "InteractiveAudio" _interactablesound)
              (goto _label))
            (:Is%20Not%20Valid
              (goto _label))))
        (:Is%20Not%20Valid
          (Class|AudioComponent|SetWaveParameter _audio "InteractiveAudio")
          (Audio|Components|Audio|Stop _audio))))))

(fn PlayPassiveSound
  (params (NewSound :type Sound%20Wave%20Object%20Reference))
  (bind _equippedsound (Variables|Default|GetEquippedSound))
  (bind _passive (Variables|Default|GetPassive))
  (bind _passivesound (Variables|/Game/DataAssets/PDA_SoundObjects.PDA_SoundObjects_C|GetPassiveSound _equippedsound))
  (Utilities|IsValid NewSound
    (:Is%20Valid
      (Class|AudioComponent|SetWaveParameter (Variables|Default|GetPassive) "AudioLoop" NewSound))
    (:Is%20Not%20Valid
      (Utilities|IsValid _equippedsound
        (:Is%20Valid
          (Utilities|IsValid _passivesound
            (:Is%20Valid
              (Class|AudioComponent|SetWaveParameter _passive "AudioLoop" _passivesound))
            (:Is%20Not%20Valid
              _)))
        (:Is%20Not%20Valid
          (Class|AudioComponent|SetWaveParameter _passive "AudioLoop")))))
  (Audio|Components|Audio|Play _passive 0.0))

(fn CheckSoundCompatible
  (bind _returnvalue (Actor|GetComponentsByClass "/Script/Engine.StaticMeshComponent"))
  (bind _originalsound (Variables|Default|GetOriginalSound))
  (bind _equippedsound (Variables|Default|GetEquippedSound))
  (bind _returnvalue_2 (== _originalsound _equippedsound))
  (Utilities|IsValid (Variables|Default|GetEquippedSound)
    (:Is%20Valid
      (if _returnvalue_2
        (for _array_element _returnvalue
          (Rendering|SetRenderCustomDepth _array_element false))
        (Default|CallSoundCorrect)
        (else
          (for _array_element_2 _returnvalue
            (Rendering|SetCustomDepthStencilValue _array_element_2 2)))))
    (:Is%20Not%20Valid
      (for _array_element_3 _returnvalue
        (Rendering|SetCustomDepthStencilValue _array_element_3 0))))
  (bind _output_get (Variables|Default|SetbIsSoundCorrect _returnvalue_2))
  (return _output_get))

(fn SoundObjectCorrect
  (for _array_element (Actor|GetComponentsByClass "/Script/Engine.StaticMeshComponent")
    (Rendering|SetRenderCustomDepth _array_element false)))

(fn SetOverallSound
  (params (newSoundVolume :type Float%20%28double-precision%29))
  (Audio|Components|Audio|SetVolumeMultiplier (Variables|Default|GetAudio) newSoundVolume :!class /Script/Engine.AudioComponent)
  (Audio|Components|Audio|SetVolumeMultiplier (Variables|Default|GetPassive) newSoundVolume :!class /Script/Engine.AudioComponent))