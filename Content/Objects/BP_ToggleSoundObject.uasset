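; Interactable sound object actor that forwards press and hold interactions to its EquippedSound, when one is valid.
; A hold waits for the delay returned by HoldInteract, then casts the sound to PDA_ToggleSoundObjects and calls PlayPassive.
; An unconnected chain still holds toggle logic that stops or starts the Passive audio directly, but it never runs.
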(event EventBeginPlay
  (|CallParentFunction) ; This node is disabled and will not be called.\nDrag off pins to build functionality.
)

(event Collision|EventActorBeginOverlap
  (params (OtherActor :type Actor%20Object%20Reference)))

(event EventTick
  (params (DeltaSeconds :type Float%20%28single-precision%29)))

(event EventHoldInteract
  (bind _equippedsound (Variables|Default|GetEquippedSound))
  (Utilities|IsValid _equippedsound
    (:Is%20Valid
      (bind _sound_duration (Default|HoldInteract _equippedsound))
      (Utilities|FlowControl|Delay _sound_duration)
      (bind _aspda_toggle_sound_objects (Utilities|Casting|CastToPDA_ToggleSoundObjects _equippedsound))
      (Default|PlayPassive _aspda_toggle_sound_objects))))

(event EventPressInteract
  (bind _equippedsound (Variables|Default|GetEquippedSound))
  (Utilities|IsValid _equippedsound
    (:Is%20Valid
      (Default|PressInteract _equippedsound))))

(fn ConstructionScript
  (|CallParentFunction))