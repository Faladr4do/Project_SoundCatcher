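; Interactable vacuum object that plays sounds from its equipped sound data asset in response to press and hold interactions.
; Both inputs branch on the asset's gameplay tag, with press gated by a DoOnce that resets after each action.
; Press plays a one-shot or changes the station of a powered-on radio.
; Hold toggles generic, radio or light assets, stopping passive audio or starting it after the turn-on sound's delay.
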(event EventBeginPlay
  (|CallParentFunction) ; This node is disabled and will not be called.\nDrag off pins to build functionality.
)

(event Collision|EventActorBeginOverlap
  (params (OtherActor :type Actor%20Object%20Reference))
  (|CallParentFunction OtherActor) ; This node is disabled and will not be called.\nDrag off pins to build functionality.
)

(event EventTick
  (params (DeltaSeconds :type Float%20%28single-precision%29))
  (|CallParentFunction DeltaSeconds) ; This node is disabled and will not be called.\nDrag off pins to build functionality.
)

(event EventPressInteract
  (bind _equippedsound (Variables|Default|GetEquippedSound))
  (Utilities|IsValid _equippedsound
    (:Is%20Valid
      (Utilities|FlowControl|DoOnce false
        (:Completed
          (|SwitchGameplayTag (Variables|/Game/DataAssets/PDA_SoundObjects.PDA_SoundObjects_C|GetObjectType _equippedsound)
            (:SoundObjects
              (Utilities|DefaultPressAction
                (:Completed
                  _)))
            (:SoundObjects.Toggle.Radio
              (Utilities|RadioPressAction)))
          (CallFunction|ResetMyDoOnce))))))

(event EventHoldInteract
  (bind _equippedsound (Variables|Default|GetEquippedSound))
  (Utilities|IsValid _equippedsound
    (:Is%20Valid
      (|SwitchGameplayTag (Variables|/Game/DataAssets/PDA_SoundObjects.PDA_SoundObjects_C|GetObjectType _equippedsound)
        (:SoundObjects.Toggle
          (Utilities|ToggleHoldAction))
        (:SoundObjects.Toggle.Radio
          (Utilities|RadioHoldAction))
        (:SoundObjects.Toggle.Light
          (Utilities|LightHoldAction)))
      (CallFunction|ResetMyDoOnce))))

(event EventResetMyDoOnce
  (Utilities|FlowControl|DoOnce false) ; enters at Reset
)

(fn ConstructionScript
  (|CallParentFunction))